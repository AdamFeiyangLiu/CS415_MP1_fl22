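; BP_Projectile is an arrow projectile that destroys enemies and awards score to the player.
; Tick moves it along world X with a swept offset at a set speed, and a timer started on BeginPlay destroys it after a short lifetime.
; When the arrow mesh overlaps a BP_Enemy, it destroys both actors and adds points to the cached BP_Player; any other overlap stops its movement.
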(event `DestroyProjectile`
  (`/Engine/EditorBlueprintResources/StandardMacros.IsValid` self
    (:`Is Valid`
      (`self.K2_DestroyActor`))))

(event `self.ReceiveBeginPlay`
  (`KismetSystemLibrary.K2_SetTimerDelegate` (delegate `DestroyProjectile`) 2.5)
  (bind _asbp_player (cast `/Game/InfiniteMatrix/Blueprints/BP_Player` (`GameplayStatics.GetPlayerPawn` 0)))
  (set `self.PlayerRef` _asbp_player))

(event `self.ReceiveTick`
  (params (DeltaSeconds :type "Float (single-precision)"))
  (`SceneComponent.K2_AddWorldOffset` (`self.DefaultSceneRoot`) (`KismetMathLibrary.MakeVector` (* DeltaSeconds (`self.ProSpeed`))) true false))

(event `self.SK_Arrow.OnComponentBeginOverlap`
  (params (OverlappedComponent :type "PrimitiveComponent Object Reference") (OtherActor :type "Actor Object Reference") (OtherComp :type "PrimitiveComponent Object Reference") (OtherBodyIndex :type Integer) (bFromSweep :type Boolean) (SweepResult :type "HitResult Structure (by ref)"))
  (bind _playerref (`self.PlayerRef`))
  (bind _asbp_enemy (cast `/Game/InfiniteMatrix/Blueprints/BP_Enemy` OtherActor)
    (:`then`
      (bind _output_get (set `self.As BP Enemy` _asbp_enemy))
      (`self.K2_DestroyActor` _output_get)
      (set `/Game/InfiniteMatrix/Blueprints/BP_Player.Score` (+ (`/Game/InfiniteMatrix/Blueprints/BP_Player.Score` _playerref) 5) _playerref)
      (`self.K2_DestroyActor`))
    (:`CastFailed`
      (set `self.ProSpeed` 0.0))))

(fn `UserConstructionScript`)