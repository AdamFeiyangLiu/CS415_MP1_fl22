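; Health potion pickup that heals the player on contact and exists only for a short time.
; Overlapping its mesh with BP_Player adds a fixed, clamped amount to CurHP, refreshes the heart display through HeartWarpRef, then destroys the potion.
; BeginPlay starts a timer that destroys the potion after a few seconds and caches a player reference, which the overlap logic does not use.
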(event `self.ReceiveTick`
  (params (DeltaSeconds :type "Float (single-precision)")))

(event `self.SM-Potion-1.OnComponentBeginOverlap`
  (params (OverlappedComponent :type "PrimitiveComponent Object Reference") (OtherActor :type "Actor Object Reference") (OtherComp :type "PrimitiveComponent Object Reference") (OtherBodyIndex :type Integer) (bFromSweep :type Boolean) (SweepResult :type "HitResult Structure (by ref)"))
  (cast `/Game/InfiniteMatrix/Blueprints/BP_Player` OtherActor)
  (bind _output_get (set `/Game/InfiniteMatrix/Blueprints/BP_Player.CurHP` (`KismetMathLibrary.FClamp` (+ (`/Game/InfiniteMatrix/Blueprints/BP_Player.CurHP` (stale `self.ReceiveBeginPlay` _asbp_player)) 50.0) 0.0 600.0) (stale `self.ReceiveBeginPlay` _asbp_player)))
  (`/Game/InfiniteMatrix/UI/HeartUI/HeartWarpBox.UpdateHeart` (`/Game/InfiniteMatrix/Blueprints/BP_Player.HeartWarpRef` (stale `self.ReceiveBeginPlay` _asbp_player)) (/ _output_get 100.0))
  (`self.K2_DestroyActor`))

(event `self.ReceiveBeginPlay`
  (`KismetSystemLibrary.K2_SetTimerDelegate` (delegate `destroyPotion`) 5.0)
  (bind _asbp_player (cast `/Game/InfiniteMatrix/Blueprints/BP_Player` (`GameplayStatics.GetPlayerPawn` 0)))
  (set `self.As BP Player` _asbp_player))

(event `destroyPotion`
  (`/Engine/EditorBlueprintResources/StandardMacros.IsValid` self
    (:`Is Valid`
      (`self.K2_DestroyActor`))))

(fn `UserConstructionScript`)